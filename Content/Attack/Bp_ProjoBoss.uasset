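; Boss attack actor that plays a thunder sound, then briefly activates a particle effect after a one-second delay.
; A looping timer then repeatedly sphere-traces at the Zone component on the Visibility channel, with debug drawing on.
; Each hit on a Player-tagged actor subtracts Degat from the player character's Life via ChangerVie.
; Any hit result, player or not, leads to a delayed self-destroy, with damage able to repeat until then.
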(event `self.ReceiveBeginPlay`
  (`GameplayStatics.PlaySound2D` "/Game/StarterContent/Audio/Tonerre.Tonerre" 1.0 1.0 0.0 null null)
  (`KismetSystemLibrary.Delay` 1.0)
  (`ActorComponent.Activate` (`self.ParticleSystem`) true)
  (`KismetSystemLibrary.Delay` 0.2)
  (`KismetSystemLibrary.K2_SetTimerDelegate` (delegate `ultime1`) 0.1 true)
  (`ActorComponent.Activate` (`self.ParticleSystem`) false)
  (`KismetSystemLibrary.Delay` 0.1))

(event `ultime1`
  (bind _returnvalue (`SceneComponent.K2_GetComponentLocation` (`self.Zone`)))
  (bind _outhits (`KismetSystemLibrary.SphereTraceMulti` :`Start` _returnvalue :`End` _returnvalue :`Radius` 120.0 :`TraceChannel` "TraceTypeQuery1" :`DrawDebugType` "ForDuration" :`DrawTime` 0.2))
  (for _array_element _outhits
    (bind (_bblockinghit _binitialoverlap _time _distance _location _impactpoint _normal _impactnormal _physmat _hitactor) (`GameplayStatics.BreakHitResult` _array_element))
    (`/Engine/EditorBlueprintResources/StandardMacros.IsValid` _hitactor
      (:`Is Valid`
        (if (`self.ActorHasTag` _hitactor "Player")
          (bind _asbp_top_down_character (cast `/Game/TopDown/Blueprints/BP_TopDownCharacter` (`GameplayStatics.GetPlayerCharacter` 0)))
          (`/Game/TopDown/Blueprints/BP_TopDownCharacter.ChangerVie` _asbp_top_down_character (`KismetMathLibrary.FTrunc` (- (`/Game/TopDown/Blueprints/BP_TopDownCharacter.Life` _asbp_top_down_character) (`self.Degat`))))))
      (:`Is Not Valid`
        _))
    (`KismetSystemLibrary.Delay` 6.0)
    (`self.K2_DestroyActor`)))

(fn `UserConstructionScript`)