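; BP_IAenemy is an enemy character that takes damage and knockback and is destroyed when its health runs out.
; The Attack event passes damage and knockback to Damaged0, which applies a velocity-change impulse opposite the enemy's own forward vector, regardless of attacker position.
; It then subtracts damage from VieEnemy and destroys the actor at zero or below.
; No AI behavior is implemented in these graphs.
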(event `self.ReceiveBeginPlay`
  (`parent.ReceiveBeginPlay`))

(event `/Game/Attack/BPI_Attack.Attack`
  (params (Player :type "/Game/TopDown/Blueprints/BP_TopDownCharacter Object Reference") (Dmg :type Integer) (Knockback :type Integer))
  (`self.Damaged_0` Dmg Knockback))

(fn `Damaged_0`
  (params (Dmg :type Integer) (Knockback :type Integer))
  (`CharacterMovementComponent.AddImpulse` (`self.CharacterMovement`) (* (* (`self.GetActorForwardVector`) (-1.0 -1.0 -1.0)) (`KismetMathLibrary.Conv_IntToDouble` Knockback)) true)
  (set `self.VieEnemy` (- (`self.VieEnemy`) Dmg))
  (if (<= (`self.VieEnemy`) 0.0)
    (`self.K2_DestroyActor`)))

(fn `NewFunction`)

(fn `UserConstructionScript`)