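; BP_Pickup is a respawning pickup that triggers when a BP_TopDownCharacter overlaps it.
; Overlap calls EffetPickup, an empty function here that serves as the effect hook, then Desactivation hides the Scene hierarchy and disables Sphere collision.
; Desactivation starts the AttenteReactivation event, which waits DureeRespawnSec before Activation restores visibility and collision, reusing the actor instead of destroying it.
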(event `self.ReceiveActorBeginOverlap`
  (params (OtherActor :type "Actor Object Reference"))
  (bind _asbp_top_down_character (cast `/Game/TopDown/Blueprints/BP_TopDownCharacter` OtherActor))
  (`self.EffetPickup` _asbp_top_down_character)
  (`self.Desactivation`))

(event `AttenteReactivation`
  (`KismetSystemLibrary.Delay` (`self.DureeRespawnSec`))
  (`self.Activation`))

(fn `Activation`
  (`SceneComponent.SetHiddenInGame` (`self.Scene`) false true)
  (`PrimitiveComponent.SetCollisionEnabled` (`self.Sphere`) "QueryAndPhysics"))

(fn `Desactivation`
  (`SceneComponent.SetHiddenInGame` (`self.Scene`) true true)
  (`PrimitiveComponent.SetCollisionEnabled` (`self.Sphere`) "NoCollision")
  (`self.AttenteReactivation`))

(fn `EffetPickup`
  (params (Player :type "/Game/TopDown/Blueprints/BP_TopDownCharacter Object Reference")))

(fn `UserConstructionScript`)