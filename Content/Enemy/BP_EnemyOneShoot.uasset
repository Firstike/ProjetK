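; BP_EnemyOneShoot is an enemy actor that takes damage and is destroyed when its health runs out.
; The Attack event passes its damage amount to the Damaged0 function, which subtracts it from VieEnemy and destroys the actor at zero or below.
; It has no active BeginPlay, overlap or Tick logic, and the construction script only calls its parent.
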(event `/Game/Attack/BPI_Attack.Attack`
  (params (Player :type "/Game/TopDown/Blueprints/BP_TopDownCharacter Object Reference") (Dmg :type Integer))
  (`self.Damaged_0` Dmg))

(fn `Damaged_0`
  (params (Dmg :type Integer))
  (set `self.VieEnemy` (- (`self.VieEnemy`) Dmg))
  (if (<= (`self.VieEnemy`) 0.0)
    (`self.K2_DestroyActor`)))

(fn `UserConstructionScript`
  (`parent.UserConstructionScript`))