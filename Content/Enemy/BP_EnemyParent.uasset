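; Base enemy Blueprint that tracks health and destroys the actor when health runs out.
; On BeginPlay it passes itself to the VieEnemy health widget in its VieWidget component.
; The Attack event forwards incoming damage to Damaged, which subtracts it from the VieEnemy value and destroys the actor at zero or below.
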(event `self.ReceiveBeginPlay`
  (bind _asvie_enemy (cast `/Game/Widget/VieEnemy` (`WidgetComponent.GetWidget` (`self.VieWidget`))))
  (set `/Game/Widget/VieEnemy.EnemyRef` self _asvie_enemy))

(event `/Game/Attack/BPI_Attack.Attack`
  (params (Player :type "/Game/TopDown/Blueprints/BP_TopDownCharacter Object Reference") (Dmg :type Integer))
  (`self.Damaged` Dmg))

(fn `Damaged`
  (params (Dmg :type Integer))
  (set `self.VieEnemy` (- (`self.VieEnemy`) Dmg))
  (if (<= (`self.VieEnemy`) 0.0)
    (`self.K2_DestroyActor`)))

(fn `UserConstructionScript`)