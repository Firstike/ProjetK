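; BP_EnemyPara is an enemy that attacks the top-down player at range and dies when its health runs out.
; Each tick it turns its capsule toward the player and, when close enough, spawns Bp_Projo at the player's position on a fixed height, gated by a cooldown.
; Tick also pulses the Cone's horizontal scale.
; The Attack event subtracts damage from VieEnemy; its knockback impulse is zero, so the Knockback input has no effect.
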(event `self.ReceiveBeginPlay`
  (bind _asbp_top_down_character (cast `/Game/TopDown/Blueprints/BP_TopDownCharacter` (`GameplayStatics.GetPlayerCharacter` 0)))
  (set `self.As BP Top Down Character` _asbp_top_down_character)
  (`parent.ReceiveBeginPlay`))

(event `/Game/Attack/BPI_Attack.Attack`
  (params (Player :type "/Game/TopDown/Blueprints/BP_TopDownCharacter Object Reference") (Dmg :type Integer) (Knockback :type Integer))
  (`self.Damaged_0` Dmg Knockback))

(event `self.ReceiveTick`
  (params (DeltaSeconds :type "Float (single-precision)"))
  (bind (_returnvalue_x _returnvalue_y) (`KismetMathLibrary.BreakVector` (`self.K2_GetActorLocation` (`self.As BP Top Down Character`))))
  (bind (_returnvalue_x_2 _returnvalue_y_2) (`KismetMathLibrary.BreakVector` (`SceneComponent.K2_GetComponentScale` (`self.Cone`))))
  (bind (_returnvalue_x_3 _returnvalue_y_3) (`KismetMathLibrary.BreakVector` (`SceneComponent.K2_GetComponentScale` (`self.Cone`))))
  (`|ExecutionSequence`
    (:`then_0`
      (`SceneComponent.K2_SetWorldRotation` (`self.CapsuleComponent`) (`KismetMathLibrary.FindLookAtRotation` (`self.K2_GetActorLocation`) (`self.K2_GetActorLocation` (`self.As BP Top Down Character`))) false false)
      (if (< (`KismetMathLibrary.Round` (`self.GetDistanceTo` (`self.As BP Top Down Character`))) 700)
        (if (not (`self.Atk?`))
          (set `self.Atk?` true)
          (`|SpawnActorFromClass` "/Game/Attack/Bp_Projo.Bp_Projo_C" (`KismetMathLibrary.MakeTransform` (`KismetMathLibrary.MakeVector` _returnvalue_x _returnvalue_y 94.0)) "Undefined" "OverrideRootScale" null null)
          (`KismetSystemLibrary.Delay` 1.5)
          (set `self.Atk?` false))))
    (:`then_1`
      (if (`self.Anim?`)
        (`SceneComponent.SetWorldScale3D` (`self.Cone`) (`KismetMathLibrary.MakeVector` (+ _returnvalue_x_3 0.05) (+ _returnvalue_y_3 0.05) 1.0))
        (if (>= _returnvalue_x_3 1.6)
          (set `self.Anim?` false))
        (else
          (`SceneComponent.SetWorldScale3D` (`self.Cone`) (`KismetMathLibrary.MakeVector` (- _returnvalue_x_2 0.05) (- _returnvalue_y_2 0.05) 1.0))
          (if (>= 0.6 _returnvalue_x_2)
            (set `self.Anim?` true)))))))

(fn `Damaged_0`
  (params (Dmg :type Integer) (Knock :type Integer))
  (`CharacterMovementComponent.AddImpulse` (`self.CharacterMovement`) (0.0 0.0 0.0) true)
  (set `self.VieEnemy` (- (`self.VieEnemy`) Dmg))
  (if (<= (`self.VieEnemy`) 0.0)
    (`self.K2_DestroyActor`)))

(fn `UserConstructionScript`
  (`parent.UserConstructionScript`))