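; Tamamo boss enemy that runs a numbered phase fight, advancing whenever damage empties its health and refilling it until the finale.
; Tick pins it to a location per phase and drives Delay-gated attacks: corner fireballs, then scripted center projectile barrages while it is off-arena, then both combined.
; Barrage completion also advances phases 5 and 6.
; A pulsing cone expands in phase 11, with staggered Niagara explosions and sounds as the finale.
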(event `self.ReceiveBeginPlay`
  (bind _asbp_top_down_character (cast `/Game/TopDown/Blueprints/BP_TopDownCharacter` (`GameplayStatics.GetPlayerCharacter` 0)))
  (set `self.As BP Top Down Character` _asbp_top_down_character)
  (`parent.ReceiveBeginPlay`))

(event `/Game/Attack/BPI_Attack.Attack`
  (params (Player :type "/Game/TopDown/Blueprints/BP_TopDownCharacter Object Reference") (Dmg :type Integer) (Knockback :type Integer))
  (`self.Damaged_0` Dmg Knockback))

(event `self.ReceiveTick`
  (params (DeltaSeconds :type "Float (single-precision)"))
  (bind _phase (`self.Phase`))
  (bind _phase_2 (`self.Phase`))
  (bind _delayeclair (`self.DelayEclair`))
  (bind _phase_3 (`self.Phase`))
  (bind _phase_4 (`self.Phase`))
  (bind (_returnvalue_x _returnvalue_y) (`KismetMathLibrary.BreakVector` (`SceneComponent.K2_GetComponentScale` (`self.Cone`))))
  (bind (_returnvalue_x_2 _returnvalue_y_2) (`KismetMathLibrary.BreakVector` (`SceneComponent.K2_GetComponentScale` (`self.Cone`))))
  (bind (_returnvalue_x_3 _returnvalue_y_3) (`KismetMathLibrary.BreakVector` (`SceneComponent.K2_GetComponentScale` (`self.Cone`))))
  (bind (_returnvalue_x_4 _returnvalue_y_4 _returnvalue_z) (`KismetMathLibrary.BreakVector` (`SceneComponent.K2_GetComponentLocation` (`self.CapsuleComponent`))))
  (`|ExecutionSequence`
    (:`then_0`
      ;[1 1 1] TpPhase1-4
      (if (or (== _phase_4 1) (== _phase_4 7))
        (`SceneComponent.K2_SetWorldLocation` (`self.CapsuleComponent`) (`KismetMathLibrary.MakeVector` 2636.0 357.0 _returnvalue_z) false true)
        (elif (or (== _phase 2) (== _phase 8))
          (`SceneComponent.K2_SetWorldLocation` (`self.CapsuleComponent`) (`KismetMathLibrary.MakeVector` 2636.0 1851.0 _returnvalue_z) false true)
          (elif (or (== _phase_2 3) (== _phase_2 9))
            (`SceneComponent.K2_SetWorldLocation` (`self.CapsuleComponent`) (`KismetMathLibrary.MakeVector` 1091.0 1851.0 _returnvalue_z) false true)
            (elif (or (== _phase_3 4) (== _phase_3 10))
              (`SceneComponent.K2_SetWorldLocation` (`self.CapsuleComponent`) (`KismetMathLibrary.MakeVector` 1091.0 357.0 _returnvalue_z) false true)
              (elif (== (`self.Phase`) 5)
                (`SceneComponent.K2_SetWorldLocation` (`self.CapsuleComponent`) (4000.0 4000.0 0.0) false true)
                (elif (== (`self.Phase`) 11)
                  (`SceneComponent.K2_SetWorldLocation` (`self.CapsuleComponent`) (2036.0 1128.0 200.0) false true))))))))
    (:`then_1`
      (if (<= (`self.Phase`) 4)
        ;[1 1 1] Phase1-4
        (if (`self.Atk?`) :!label _label
          (set `self.Atk?` false)
          (`|SpawnActorFromClass` "/Game/Attack/Test/FireballBoss.FireballBoss_C" (`KismetMathLibrary.MakeTransform` (`SceneComponent.K2_GetComponentLocation` (`self.AtkPoint`)) (`SceneComponent.K2_GetComponentRotation` (`self.AtkPoint`))) "Undefined" "OverrideRootScale" null null)
          (`GameplayStatics.PlaySound2D` "/Game/StarterContent/Audio/Explosion01.Explosion01" 1.0 1.0 0.0 null null)
          (`KismetSystemLibrary.Delay` 1.5)
          (set `self.Atk?` true))
        (elif (and (>= (`self.Phase`) 7) (<= (`self.Phase`) 10))
          (`|ExecutionSequence`
            (:`then_0`
              (goto _label))
            (:`then_1`
              (set `self.DelayEclair` 1.0)
              (set `self.Delay Boom` 1.5)
              (if (`self.Atk5`) :!label _label_2
                (set `self.Atk5` false)
                ;[1 1 1] Phase5
                (`KismetSystemLibrary.Delay` 0.5)
                (`|SpawnActorFromClass` "/Game/Attack/Bp_ProjoBoss.Bp_ProjoBoss_C" (`KismetMathLibrary.MakeTransform` (2036.0 1128.0 165.0) (struct :`Yaw` 180.0)) "Undefined" "OverrideRootScale" null null)
                (`KismetSystemLibrary.Delay` _delayeclair)
                (`|SpawnActorFromClass` "/Game/Attack/Bp_ProjoBoss.Bp_ProjoBoss_C" (`KismetMathLibrary.MakeTransform` (2036.0 1128.0 165.0) (struct :`Yaw` 80.0)) "Undefined" "OverrideRootScale" null null)
                (`KismetSystemLibrary.Delay` _delayeclair)
                (`|SpawnActorFromClass` "/Game/Attack/Bp_ProjoBoss.Bp_ProjoBoss_C" (`KismetMathLibrary.MakeTransform` (2036.0 1128.0 165.0) (struct :`Yaw` 10.0)) "Undefined" "OverrideRootScale" null null)
                (`KismetSystemLibrary.Delay` (`self.DelayEclair`))
                (`|SpawnActorFromClass` "/Game/Attack/Bp_ProjoBoss.Bp_ProjoBoss_C" (`KismetMathLibrary.MakeTransform` (2036.0 1128.0 165.0) (struct :`Yaw` 75.0)) "Undefined" "OverrideRootScale" null null)
                (`KismetSystemLibrary.Delay` (`self.DelayEclair`))
                (`|SpawnActorFromClass` "/Game/Attack/Bp_ProjoBoss.Bp_ProjoBoss_C" (`KismetMathLibrary.MakeTransform` (2036.0 1128.0 165.0) (struct :`Yaw` 280.0)) "Undefined" "OverrideRootScale" null null)
                (`KismetSystemLibrary.Delay` (`self.DelayEclair`))
                (`|SpawnActorFromClass` "/Game/Attack/Bp_ProjoBoss.Bp_ProjoBoss_C" (`KismetMathLibrary.MakeTransform` (2036.0 1128.0 165.0) (struct :`Yaw` 320.0)) "Undefined" "OverrideRootScale" null null)
                (`KismetSystemLibrary.Delay` (`self.DelayEclair`))
                (`|SpawnActorFromClass` "/Game/Attack/Bp_ProjoBoss.Bp_ProjoBoss_C" (`KismetMathLibrary.MakeTransform` (2036.0 1128.0 165.0) (struct :`Yaw` 215.0)) "Undefined" "OverrideRootScale" null null)
                (`KismetSystemLibrary.Delay` (`self.DelayEclair`))
                (`|SpawnActorFromClass` "/Game/Attack/Bp_ProjoBoss.Bp_ProjoBoss_C" (`KismetMathLibrary.MakeTransform` (2036.0 1128.0 165.0)) "Undefined" "OverrideRootScale" null null)
                (`KismetSystemLibrary.Delay` (`self.DelayEclair`))
                (`|SpawnActorFromClass` "/Game/Attack/Bp_ProjoBoss.Bp_ProjoBoss_C" (`KismetMathLibrary.MakeTransform` (2036.0 1128.0 165.0) (struct :`Yaw` 330.0)) "Undefined" "OverrideRootScale" null null)
                (`KismetSystemLibrary.Delay` (`self.DelayEclair`))
                (`|SpawnActorFromClass` "/Game/Attack/Bp_ProjoBoss.Bp_ProjoBoss_C" (`KismetMathLibrary.MakeTransform` (2036.0 1128.0 165.0) (struct :`Yaw` 180.0)) "Undefined" "OverrideRootScale" null null)
                (`KismetSystemLibrary.Delay` (`self.DelayEclair`))
                (`|SpawnActorFromClass` "/Game/Attack/Bp_ProjoBoss.Bp_ProjoBoss_C" (`KismetMathLibrary.MakeTransform` (2036.0 1128.0 165.0) (struct :`Yaw` 200.0)) "Undefined" "OverrideRootScale" null null)
                (`KismetSystemLibrary.Delay` (`self.DelayEclair`))
                (`|SpawnActorFromClass` "/Game/Attack/Bp_ProjoBoss.Bp_ProjoBoss_C" (`KismetMathLibrary.MakeTransform` (2036.0 1128.0 165.0) (struct :`Yaw` 130.0)) "Undefined" "OverrideRootScale" null null)
                (`KismetSystemLibrary.Delay` (`self.DelayEclair`))
                (if (== (`self.Phase`) 5)
                  (set `self.Phase` 6)
                  (else
                    (`|SpawnActorFromClass` "/Game/Attack/Bp_ProjoBoss2.Bp_ProjoBoss2_C" (`KismetMathLibrary.MakeTransform` (2036.0 1128.0 165.0) (struct :`Yaw` 90.0)) "Undefined" "OverrideRootScale" null null :!label _label_3)
                    (`KismetSystemLibrary.Delay` (`self.Delay Boom`))
                    (`|SpawnActorFromClass` "/Game/Attack/Bp_ProjoBoss2.Bp_ProjoBoss2_C" (`KismetMathLibrary.MakeTransform` (2036.0 1128.0 165.0) (struct)) "Undefined" "OverrideRootScale" null null)
                    (`KismetSystemLibrary.Delay` (`self.Delay Boom`))
                    (`|SpawnActorFromClass` "/Game/Attack/Bp_ProjoBoss2.Bp_ProjoBoss2_C" (`KismetMathLibrary.MakeTransform` (2036.0 1128.0 165.0) (struct :`Yaw` 220.0)) "Undefined" "OverrideRootScale" null null)
                    (`KismetSystemLibrary.Delay` (`self.Delay Boom`))
                    (`|SpawnActorFromClass` "/Game/Attack/Bp_ProjoBoss2.Bp_ProjoBoss2_C" (`KismetMathLibrary.MakeTransform` (2036.0 1128.0 165.0) (struct :`Yaw` 300.0)) "Undefined" "OverrideRootScale" null null)
                    (`KismetSystemLibrary.Delay` (`self.Delay Boom`))
                    (`|SpawnActorFromClass` "/Game/Attack/Bp_ProjoBoss2.Bp_ProjoBoss2_C" (`KismetMathLibrary.MakeTransform` (2036.0 1128.0 165.0) (struct :`Yaw` 50.0)) "Undefined" "OverrideRootScale" null null)
                    (`KismetSystemLibrary.Delay` (`self.Delay Boom`))
                    (`|SpawnActorFromClass` "/Game/Attack/Bp_ProjoBoss2.Bp_ProjoBoss2_C" (`KismetMathLibrary.MakeTransform` (2036.0 1128.0 165.0) (struct :`Yaw` 150.0)) "Undefined" "OverrideRootScale" null null)
                    (`KismetSystemLibrary.Delay` (`self.Delay Boom`))
                    (`|SpawnActorFromClass` "/Game/Attack/Bp_ProjoBoss2.Bp_ProjoBoss2_C" (`KismetMathLibrary.MakeTransform` (2036.0 1128.0 165.0) (struct :`Yaw` 110.0)) "Undefined" "OverrideRootScale" null null)
                    (`KismetSystemLibrary.Delay` (`self.Delay Boom`))
                    (`|SpawnActorFromClass` "/Game/Attack/Bp_ProjoBoss2.Bp_ProjoBoss2_C" (`KismetMathLibrary.MakeTransform` (2036.0 1128.0 165.0) (struct :`Yaw` 30.0)) "Undefined" "OverrideRootScale" null null)
                    (`KismetSystemLibrary.Delay` 1.5)
                    (if (== (`self.Phase`) 6)
                      (set `self.Phase` 7)
                      (`SceneComponent.K2_SetWorldLocation` (`self.CapsuleComponent`) (2636.0 357.0 200.0) false true)
                      (set `self.Atk5` true)
                      (else
                        (set `self.Atk5` true))))))))
          (elif (== (`self.Phase`) 5)
            (goto _label_2)
            (elif (== (`self.Phase`) 6)
              (if (not (`self.atk6`))
                (set `self.atk6` true)
                (goto _label_3))
              (elif (== (`self.Phase`) 11)
                ;[1 1 1] Phase11
                (`KismetSystemLibrary.Delay` 0.2)
                (if (not (`self.Fin`))
                  (set `self.Fin` true)
                  (`|ExecutionSequence`
                    (:`then_0`
                      (`SceneComponent.SetWorldScale3D` (`self.Cone`) (`KismetMathLibrary.MakeVector` (+ _returnvalue_x_3 0.05) (+ _returnvalue_y_3 0.05) 2.0) :!label _label_4)
                      (if (>= _returnvalue_x_3 5.0)
                        (set `self.Fin2` true)
                        (else
                          (`KismetSystemLibrary.Delay` 0.02)
                          (goto _label_4))))
                    (:`then_1`
                      _))
                  (`KismetSystemLibrary.Delay` 0.5)
                  (`|ExecutionSequence`
                    (:`then_0`
                      (`ActorComponent.Activate` (`self.Niagara`) false :!label _label_5)
                      (`GameplayStatics.PlaySound2D` "/Game/StarterContent/Audio/Explosion01.Explosion01" 1.0 1.0 0.0 null null :!label _label_6))
                    (:`then_1`
                      (`KismetSystemLibrary.Delay` 0.2)
                      (goto _label_5))
                    (:`then_2`
                      (`KismetSystemLibrary.Delay` 0.5)
                      (`ActorComponent.Activate` (`self.Niagara1`) false)
                      (goto _label_6))
                    (:`then_3`
                      (`KismetSystemLibrary.Delay` 0.6)
                      (`ActorComponent.Activate` (`self.Niagara2`) false)
                      (goto _label_6))
                    (:`then_4`
                      (`KismetSystemLibrary.Delay` 0.8)
                      (`ActorComponent.Activate` (`self.Niagara3`) false)
                      (goto _label_6))
                    (:`then_5`
                      (`KismetSystemLibrary.Delay` 1.5)
                      (if (`self.Fin`)
                        (`ActorComponent.Activate` (`self.Niagara4`) false)
                        (`GameplayStatics.PlaySound2D` "/Game/StarterContent/Audio/Explosion02.Explosion02" 1.0 1.0 0.0 null null)))
                    (:`then_6`
                      (if (`self.Fin`)
                        (`KismetSystemLibrary.Delay` 3.0)))))))))))
    (:`then_2`
      (if (== (`self.Phase`) 11)
        _
        (elif (`self.Anim?`)
          (`SceneComponent.SetWorldScale3D` (`self.Cone`) (`KismetMathLibrary.MakeVector` (+ _returnvalue_x 0.05) (+ _returnvalue_y 0.05) 2.0))
          (if (>= _returnvalue_x 1.6)
            (set `self.Anim?` false))
          (else
            (`SceneComponent.SetWorldScale3D` (`self.Cone`) (`KismetMathLibrary.MakeVector` (- _returnvalue_x_2 0.05) (- _returnvalue_y_2 0.05) 2.0))
            (if (>= 0.6 _returnvalue_x_2)
              (set `self.Anim?` true))))))))

(fn `Damaged_0`
  (params (Dmg :type Integer) (Knock :type Integer))
  (`CharacterMovementComponent.AddImpulse` (`self.CharacterMovement`) (0.0 0.0 0.0) true)
  (set `self.VieEnemy` (- (`self.VieEnemy`) Dmg))
  (if (<= (`self.VieEnemy`) 0.0)
    (set `self.Phase` (+ (`self.Phase`) 1))
    (if (>= (`self.Phase`) 11)
      (set `self.VieEnemy` -1.0)
      (elif (>= (`self.Phase`) 5)
        (set `self.VieEnemy` 80.0)
        (else
          (set `self.VieEnemy` 50.0))))))

(fn `UserConstructionScript`
  (`parent.UserConstructionScript`))