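; BP_Champ is a farm field that grows metal crops (gold, steel, mithril) for resource harvesting.
; Interagir opens the ChoixPlant widget when the field is empty, otherwise calls PousseUpgrade to advance or harvest.
; SpawnPlant applies the given material and advances growth through two Delays, swapping three meshes' visibility.
; PousseUpgrade plays Niagara effects, spotlights ripe crops, and on harvest credits the BP_TopDownGameMode resource matching the material.
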(event `/Game/ObjetInteraction/BPI_Interaction.Interagir`
  (params (Player :type "/Game/TopDown/Blueprints/BP_TopDownCharacter Object Reference"))
  ;[1 1 1] Interact
  (set `self.BP_Champ` self)
  (if (== (`self.NiveauPousse`) 0)
    (`self.Plant`)
    (else
      (`self.PousseUpgrade` (`self.NiveauPousse`)))))

(event `SpawnPlant`
  (params (Material :type "MaterialInterface Object Reference"))
  ;[1 1 1] SPawnPlant
  (bind _output_get (set `self.MaterialPlant` Material))
  (`PrimitiveComponent.SetMaterial` (`self.Pousse1`) 0 _output_get)
  (`PrimitiveComponent.SetMaterial` (`self.Pousse2`) 0 _output_get)
  (`PrimitiveComponent.SetMaterial` (`self.Pousse3`) 0 _output_get)
  (`SceneComponent.SetVisibility` (`self.Pousse1`) true false)
  (set `self.NiveauPousse` 1)
  (`KismetSystemLibrary.Delay` 10.0)
  (`self.PousseUpgrade` (`self.NiveauPousse`))
  (`KismetSystemLibrary.Delay` 15.0)
  (`self.PousseUpgrade` (`self.NiveauPousse`)))

(fn `Plant`
  (bind _returnvalue (`|CreateWidget` "/Game/Widget/Farming/ChoixPlant.ChoixPlant_C"))
  (set `/Game/Widget/Farming/ChoixPlant.BP_ChampWdg` (`self.BP_Champ`) _returnvalue)
  (`UserWidget.AddToViewport` _returnvalue 0))

(fn `PousseUpgrade`
  (params (NiveauPousse :type Integer))
  (if (== NiveauPousse 1)
    (`SceneComponent.SetVisibility` (`self.Pousse1`) false false)
    (`SceneComponent.SetVisibility` (`self.Pousse2`) true false)
    (set `self.NiveauPousse` (+ (`self.NiveauPousse`) 1))
    (`ActorComponent.Activate` (`self.Nia_RecolteUp`) true)
    (elif (== NiveauPousse 2)
      (`SceneComponent.SetVisibility` (`self.Pousse2`) false false)
      (`SceneComponent.SetVisibility` (`self.Pousse3`) true false)
      (set `self.NiveauPousse` (+ (`self.NiveauPousse`) 1))
      (`ActorComponent.Activate` (`self.Nia_RecolteUp`) true)
      (`SceneComponent.SetVisibility` (`self.SpotLight`) true false)
      (else
        ;[1 1 1] Recolte
        (`SceneComponent.SetVisibility` (`self.Pousse3`) false false)
        (set `self.NiveauPousse` 0)
        (if (== (`self.MaterialPlant`) "/Game/StarterContent/Materials/M_Metal_Gold.M_Metal_Gold")
          (bind _asbp_top_down_game_mode (cast `/Game/TopDown/Blueprints/BP_TopDownGameMode` (`GameplayStatics.GetGameMode`)))
          (set `/Game/TopDown/Blueprints/BP_TopDownGameMode.Gold` (+ (`/Game/TopDown/Blueprints/BP_TopDownGameMode.Gold` _asbp_top_down_game_mode) 3) _asbp_top_down_game_mode)
          (`ActorComponent.Activate` (`self.Nia_Recolte`) true :!label _label)
          (`SceneComponent.SetVisibility` (`self.SpotLight`) false false)
          (elif (== (`self.MaterialPlant`) "/Game/StarterContent/Materials/M_Metal_Steel.M_Metal_Steel")
            (bind _asbp_top_down_game_mode_2 (cast `/Game/TopDown/Blueprints/BP_TopDownGameMode` (`GameplayStatics.GetGameMode`)))
            (set `/Game/TopDown/Blueprints/BP_TopDownGameMode.Iron` (+ (`/Game/TopDown/Blueprints/BP_TopDownGameMode.Iron` _asbp_top_down_game_mode_2) 3) _asbp_top_down_game_mode_2)
            (goto _label)
            (elif (== (`self.MaterialPlant`) "/Game/MaterialCustom/M_Metal_Mithril.M_Metal_Mithril")
              (bind _asbp_top_down_game_mode_3 (cast `/Game/TopDown/Blueprints/BP_TopDownGameMode` (`GameplayStatics.GetGameMode`)))
              (set `/Game/TopDown/Blueprints/BP_TopDownGameMode.Mithril` (+ (`/Game/TopDown/Blueprints/BP_TopDownGameMode.Mithril` _asbp_top_down_game_mode_3) 3) _asbp_top_down_game_mode_3)
              (goto _label)
              (else
                (`KismetSystemLibrary.PrintString` "aled")))))))))

(fn `UserConstructionScript`)